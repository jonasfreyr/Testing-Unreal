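; Destructible wall built as a dynamic mesh box from Size, with complex-as-simple collision, that gets holes cut in it by fast impacts.
; BeginPlay prepares a reusable sphere-box cutter mesh.
; The Destruction event ignores slow hits, otherwise boolean-subtracts the cutter, stretched into a long shaft aligned to the hit-to-exit line.
; Impact speed sets the cutter's offset along the surface normal, shrinking as speed rises.
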(event EventBeginPlay
  (bind _returnvalue (DynamicMeshActor|AllocateComputeMesh))
  (bind _returnvalue_2 (Class|GeometryScriptLibraryMeshPrimitiveFunctions|AppendSphereBox :TargetMesh _returnvalue :Radius 25.0 :Debug 0))
  (Variables|Default|SetProjectile _returnvalue_2))

(event Events|EventOnRebuildGeneratedMesh
  (params (TargetMesh :type Dynamic%20Mesh%20Object%20Reference))
  (bind _size (Variables|Default|GetSize))
  (bind _output_get (Variables|Default|SetTarget%20Mesh TargetMesh))
  (Class|GeometryScriptLibraryMeshPrimitiveFunctions|AppendBox :TargetMesh _output_get :DimensionX (.x _size) :DimensionY (.y _size) :DimensionZ (.z _size) :Debug 0)
  (Class|DynamicMeshComponent|EnableComplexasSimpleCollision (Variables|DynamicMeshActor|GetDynamicMeshComponent)))

(event EventDestruction
  (params (Hit :type Hit%20Result%20Structure) (Velocity :type Vector :default "0, 0, 0") (Hit%20location :type Vector :default "0, 0, 0") (Exit%20location :type Vector :default "0, 0, 0"))
  (bind (_bblockinghit _binitialoverlap _time _distance _location _impactpoint _normal _impactnormal) (Collision|BreakHitResult Hit))
  (Variables|Default|SetSpeed (Math|Vector|VectorLength Velocity))
  (if (> (Variables|Default|GetSpeed) 1.5e+03)
    (Utilities|IsValid (Variables|Default|GetProjectile)
      (:Is%20Valid
        (GeometryScript|Booleans|ApplyMeshBoolean :TargetMesh (Variables|Default|GetTarget%20Mesh) :ToolMesh (Variables|Default|GetProjectile) :ToolTransform (Math|Transform|MakeTransform (Math|Transform|InverseTransformLocation (Transformation|GetWorldTransform (Variables|DynamicMeshActor|GetDynamicMeshComponent)) (+ _impactpoint (* _impactnormal (Math|Float|MapRangeClamped (Variables|Default|GetSpeed) 1.5e+03 3e+03 25.0 0.0)))) (Math|Conversions|RotationFromXVector (- Hit%20location Exit%20location)) "100.000000,1.000000,1.000000") :Operation "Subtract" :Debug 0)))))

(fn ConstructionScript)